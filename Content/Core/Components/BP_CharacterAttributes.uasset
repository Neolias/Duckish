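; Player attributes component that drains health over time, tracks saved friends and manages crosshair, attribute, pause and game-over widgets.
; BeginPlay creates the HUD and starts a looping timer that subtracts damage and broadcasts the new health.
; Tick pauses into game over at zero health; Escape or P opens the pause menu, both enabling the cursor.
; OnFriendSaved broadcasts the FriendsSaved value without changing it.
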(event `Key|Escape`
  (params (Key :type "Key Structure"))
  (:`Pressed`
    (`GameplayStatics.SetGamePaused` true :!label _label)
    (bind _returnvalue (`|CreateWidget` "/Game/UI/pausemenu.pausemenu_C"))
    (`UserWidget.AddToViewport` _returnvalue 0)
    (`WidgetBlueprintLibrary.SetInputMode_GameAndUIEx` (`GameplayStatics.GetPlayerController` 0) null "DoNotLock" false :!label _label_2)
    (set `PlayerController.bShowMouseCursor` true (`GameplayStatics.GetPlayerController` 0))))

(event `Key|P`
  (params (Key :type "Key Structure"))
  (:`Pressed`
    (goto _label)))

(event `OnFriendSaved`
  (`self.FriendSaved` (`self.FriendsSaved`)))

(event `self.ReceiveTick`
  (params (DeltaSeconds :type "Float (single-precision)"))
  (if (<= (`self.Health`) 0.0)
    (`WidgetLayoutLibrary.RemoveAllWidgets`)
    (`GameplayStatics.SetGamePaused` true)
    (bind _returnvalue (`|CreateWidget` "/Game/UI/WBP_GameOver.WBP_GameOver_C"))
    (`UserWidget.AddToViewport` _returnvalue 0)
    (goto _label_2)))

(event `self.ReceiveBeginPlay`
  (bind _damagerate (`self.DamageRate`))
  (`KismetSystemLibrary.K2_SetTimerDelegate` (delegate `reduceHealth`) _damagerate true false (* _damagerate -1.0))
  (bind _returnvalue (`|CreateWidget` "/Game/Core/UI/WBP_PlayerCrosshair.WBP_PlayerCrosshair_C"))
  (`UserWidget.AddToViewport` _returnvalue 0)
  (bind _returnvalue_2 (`|CreateWidget` "/Game/Core/UI/WBP_playerAttributes.WBP_playerAttributes_C" (`GameplayStatics.GetPlayerController` 0)))
  (`UserWidget.AddToViewport` _returnvalue_2 0))

(event `reduceHealth`
  (bind _output_get (set `self.Health` (- (`self.Health`) (`self.damageAmount`))))
  (`self.WhenDamage` _output_get))
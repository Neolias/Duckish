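; BP_FishWaypoint is a bubble-material waypoint actor representing a friend that can be saved or killed.
; On BeginPlay it applies bubble and outline materials and binds any incoming damage to BecomeDead, which sets IsDead.
; BecomeSaved calls its parent, zeroes the red material parameters, and, the first time only, increments the player pawn's FriendsSaved count and fires OnFriendSaved.
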(event `self.BecomeSaved`
  (bind _staticmeshcomponent (`self.StaticMeshComponent`))
  (`parent.BecomeSaved`)
  (`MeshComponent.SetScalarParameterValueOnMaterials` _staticmeshcomponent "RedAmount" 0.0)
  (`MeshComponent.SetScalarParameterValueOnMaterials` _staticmeshcomponent "RedAmountB" 0.0)
  (bind _asbp_player_pawn (cast `/Game/Core/Characters/Player/BP_PlayerPawn` (`GameplayStatics.GetPlayerPawn` 0)))
  (if (not (`self.bIsSaved`))
    (bind _bp_characterattributes (`/Game/Core/Characters/Player/BP_PlayerPawn.BP_CharacterAttributes` _asbp_player_pawn))
    (set `/Game/Core/Components/BP_CharacterAttributes.FriendsSaved` (+ (`/Game/Core/Components/BP_CharacterAttributes.FriendsSaved` _bp_characterattributes) 1) _bp_characterattributes)
    (`/Game/Core/Components/BP_CharacterAttributes.OnFriendSaved` _bp_characterattributes)
    (set `self.bIsSaved` true)))

(event `self.ReceiveBeginPlay`
  (bind _staticmeshcomponent (`self.StaticMeshComponent`))
  (add `Actor.OnTakeAnyDamage` (delegate `BecomeDead`))
  (`PrimitiveComponent.SetMaterial` _staticmeshcomponent 1 "/Game/Art/Materials/MI_BubbleOutline.MI_BubbleOutline")
  (`PrimitiveComponent.SetMaterial` _staticmeshcomponent 0 "/Game/Art/Materials/MI_Bubble.MI_Bubble"))

(event `BecomeDead`
  (params (DamagedActor :type "Actor Object Reference") (Damage :type "Float (single-precision)") (DamageType :type "DamageType Object Reference") (InstigatedBy :type "Controller Object Reference") (DamageCauser :type "Actor Object Reference"))
  (set `self.IsDead` true))

(fn `UserConstructionScript`)